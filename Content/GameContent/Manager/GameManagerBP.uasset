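; Game-wide manager that holds persistent user data, sound volume settings and a one-time logo-finished flag.
; On Init it loads the UserDataBP save from its slot or creates a new one; writing back happens only through SaveUserData.
; Volume setters clamp main, BGM, voice and effect levels above zero, store them and apply sound mix class overrides.
; InitSound reapplies only the main and BGM volumes.
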(event `self.ReceiveInit`
  (`self.LoadUserData`))

(fn `GetBGMSoundVolume`
  (returns (bgmSoundVolume :type "Float (double-precision)"))
  (return (`/Game/GameContent/Manager/UserDataBP.bgmSoundVolume` (`self.userData`))))

(fn `GetEffectSoundVolume`
  (returns (effectSoundVolume :type "Float (double-precision)"))
  (return (`/Game/GameContent/Manager/UserDataBP.effectSoundVolume` (`self.userData`))))

(fn `GetIsLogoFinish`
  (returns (isLogoFinish :type Boolean))
  (return (`self.isLogoFinish`)))

(fn `GetMainSoundVolume`
  (returns (mainSoundVolume :type "Float (double-precision)"))
  (return (`/Game/GameContent/Manager/UserDataBP.mainSoundVolume` (`self.userData`))))

(fn `GetVoiceSoundVolume`
  (returns (voiceSoundVolume :type "Float (double-precision)"))
  (return (`/Game/GameContent/Manager/UserDataBP.voiceSoundVolume` (`self.userData`))))

(fn `InitSound`
  (bind _mainsoundvolume (`self.GetMainSoundVolume`))
  (`self.SetMainSoundVolume` _mainsoundvolume)
  (bind _bgmsoundvolume (`self.GetBGMSoundVolume`))
  (`self.SetBGMSoundVolume` _bgmsoundvolume))

(fn `LoadUserData`
  (bind _returnvalue (`GameplayStatics.LoadGameFromSlot` (`self.userDataFileName`)))
  (`/Engine/EditorBlueprintResources/StandardMacros.IsValid` _returnvalue
    (:`Is Valid`
      (bind _asuser_data_bp (cast `/Game/GameContent/Manager/UserDataBP` _returnvalue))
      (set `self.userData` _asuser_data_bp))
    (:`Is Not Valid`
      (bind _returnvalue_2 (`GameplayStatics.CreateSaveGameObject` "/Game/GameContent/Manager/UserDataBP.UserDataBP_C"))
      (set `self.userData` _returnvalue_2))))

(fn `LogoFinish`
  (if (not (`self.isLogoFinish`))
    (set `self.isLogoFinish` true)))

(fn `SaveUserData`
  (`GameplayStatics.SaveGameToSlot` (`self.userData`) (`self.userDataFileName`)))

(fn `SetBGMSoundVolume`
  (params (bgmSoundVolume :type "Float (double-precision)"))
  (bind _output_get (set `/Game/GameContent/Manager/UserDataBP.bgmSoundVolume` (`KismetMathLibrary.FClamp` bgmSoundVolume 0.01) (`self.userData`)))
  (`GameplayStatics.SetSoundMixClassOverride` (`self.mainSoundMix`) (`self.bgmSoundClass`) _output_get 1.0 0.0))

(fn `SetEffectSoundVolume`
  (params (effectSoundVolume :type "Float (double-precision)"))
  (bind _output_get (set `/Game/GameContent/Manager/UserDataBP.effectSoundVolume` (`KismetMathLibrary.FClamp` effectSoundVolume 0.01) (`self.userData`)))
  (`GameplayStatics.SetSoundMixClassOverride` (`self.mainSoundMix`) (`self.effectSoundClass`) _output_get 1.0 0.0))

(fn `SetMainSoundVolume`
  (params (mainSoundVolume :type "Float (double-precision)"))
  (bind _output_get (set `/Game/GameContent/Manager/UserDataBP.mainSoundVolume` (`KismetMathLibrary.FClamp` mainSoundVolume 0.01) (`self.userData`)))
  (`GameplayStatics.SetSoundMixClassOverride` (`self.mainSoundMix`) (`self.mainSoundClass`) _output_get 1.0 0.0))

(fn `SetVoiceSoundVolume`
  (params (voiceSoundVolume :type "Float (double-precision)"))
  (bind _output_get (set `/Game/GameContent/Manager/UserDataBP.voiceSoundVolume` (`KismetMathLibrary.FClamp` voiceSoundVolume 0.01) (`self.userData`)))
  (`GameplayStatics.SetSoundMixClassOverride` (`self.mainSoundMix`) (`self.voiceSoundClass`) _output_get 1.0 0.0))